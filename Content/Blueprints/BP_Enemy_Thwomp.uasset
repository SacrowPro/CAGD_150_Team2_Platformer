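; BP_Enemy_Thwomp is a Thwomp-style enemy for a side-scroller, with its player-crushing behavior unfinished.
; A Cube hit whose impact point exactly equals the ThwompHurtbox location (zero tolerance) casts and stores the side-scroller character, then only prints debug text.
; BeginPlay caches BP_GameInstance for a disconnected chain that would flatten the character, wait, then call TakeDamage on the game instance.
; The file contains no movement logic.
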(event `self.Cube.OnComponentHit`
  (params (HitComponent :type "PrimitiveComponent Object Reference") (OtherActor :type "Actor Object Reference") (OtherComp :type "PrimitiveComponent Object Reference") (NormalImpulse :type "Vector Structure") (Hit :type "HitResult Structure (by ref)"))
  (if (== (`.ImpactPoint` (`GameplayStatics.BreakHitResult` Hit)) (`SceneComponent.K2_GetComponentLocation` (`self.ThwompHurtbox`)))
    (bind _asbp_side_scroller_character (cast `/Game/Blueprints/BP_SideScrollerCharacter` OtherActor)
      (:`then`
        (bind _output_get (set `self.As BP Side Scroller Character` _asbp_side_scroller_character))
        (`KismetSystemLibrary.PrintString` "hit sucessful"))
      (:`CastFailed`
        (`KismetSystemLibrary.PrintString` "cast failed hurtbox")))))

(event `self.ReceiveBeginPlay`
  ;[0.15 0.005781 0.005781 0.5] Get Reference to Game Instance
  (bind _asbp_game_instance (cast `/Game/Blueprints/BP_GameInstance` (`GameplayStatics.GetGameInstance`)))
  (set `self.As BP Game Instance` _asbp_game_instance))

(fn `UserConstructionScript`)