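; Thwomp enemy for the side-scroller that wiggles when the player gets near and slams down when they get closer.
; Two detection boxes drive timelines that interpolate the Thwomp between marker transforms, with an eased curve for the fall.
; An IsFalling flag keeps detection overlaps from interrupting the fall cycle.
; The hurtbox squashes the player, then after a delay applies damage through BP_GameInstance, clears Fire Flower and restores scale.
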(event `self.ReceiveBeginPlay`
  ;[0.15 0.005781 0.005781 0.5] Get Game Instance Ref
  (bind _asbp_game_instance (cast `/Game/Blueprints/BP_GameInstance` (`GameplayStatics.GetGameInstance`)))
  (set `self.As BP Game Instance` _asbp_game_instance))

(event `self.DetectBox.OnComponentBeginOverlap`
  (params (OverlappedComponent :type "PrimitiveComponent Object Reference") (OtherActor :type "Actor Object Reference") (OtherComp :type "PrimitiveComponent Object Reference") (OtherBodyIndex :type Integer) (bFromSweep :type Boolean) (SweepResult :type "HitResult Structure (by ref)"))
  (bind _thwompwiggle1 (`self.thwompwiggle1`))
  (bind _thwompwiggle2 (`self.thwompwiggle2`))
  ;[0.15 0.005781 0.005781 0.5] When only a little bit in detect zone, Thwomp wiggles from side to side
  (if (not (`self.IsFalling`))
    (bind _asbp_side_scroller_character (cast `/Game/Blueprints/BP_SideScrollerCharacter` OtherActor))
    (set `self.As BP Side Scroller Character` _asbp_side_scroller_character)
    (bind (_direction _alphawiggle) (`Timeline|Timeline_0` :!label _label)
      (:`Update`
        (set `self.Alpha Wiggle` _alphawiggle)
        (`/Engine/EditorBlueprintResources/StandardMacros.IsValid` _thwompwiggle1
          (:`Is Valid`
            (`/Engine/EditorBlueprintResources/StandardMacros.IsValid` _thwompwiggle2
              (:`Is Valid`
                (`SceneComponent.K2_SetWorldTransform` (`self.thwomp`) (`KismetMathLibrary.TLerp` (`SceneComponent.K2_GetComponentToWorld` _thwompwiggle1) (`SceneComponent.K2_GetComponentToWorld` _thwompwiggle2) (`self.Alpha Wiggle`)) true false))
              (:`Is Not Valid`
                (`KismetSystemLibrary.PrintString` "Object Not Set" :!label _label_2))))
          (:`Is Not Valid`
            (goto _label_2)))))))

(event `self.FallingDetectBox.OnComponentEndOverlap`
  (params (OverlappedComponent :type "PrimitiveComponent Object Reference") (OtherActor :type "Actor Object Reference") (OtherComp :type "PrimitiveComponent Object Reference") (OtherBodyIndex :type Integer))
  ;[0.15 0.005781 0.005781 0.5] When only a little bit in detect zone, Thwomp wiggles from side to side
  (if (not (`self.IsFalling`))
    (bind _asbp_side_scroller_character (cast `/Game/Blueprints/BP_SideScrollerCharacter` OtherActor))
    (set `self.As BP Side Scroller Character` _asbp_side_scroller_character)
    (goto _label :!via `Stop`)))

(event `self.FallingDetectBox.OnComponentBeginOverlap`
  (params (OverlappedComponent :type "PrimitiveComponent Object Reference") (OtherActor :type "Actor Object Reference") (OtherComp :type "PrimitiveComponent Object Reference") (OtherBodyIndex :type Integer) (bFromSweep :type Boolean) (SweepResult :type "HitResult Structure (by ref)"))
  (bind _thwompstart (`self.thwompstart`))
  (bind _thwompend (`self.thwompend`))
  ;[0.1667 0 0.01204 0.5] Detects if Player moves into Falling Detect Box, sets conditions to avoid falling animation being interrupted
  (if (not (`self.IsFalling`))
    (bind _asbp_side_scroller_character (cast `/Game/Blueprints/BP_SideScrollerCharacter` OtherActor))
    (set `self.As BP Side Scroller Character` _asbp_side_scroller_character)
    (set `self.IsFalling` true)
    ;[0.15 0.005781 0.005781 0.5] When Player overlaps too far into Thwomp detect zone, Thwomp falls down, then back up slowly
    (bind (_direction _alphafall) (`Timeline|Timeline` :!via `PlayFromStart`)
      (:`Update`
        (set `self.AlphaFall` _alphafall)
        (`/Engine/EditorBlueprintResources/StandardMacros.IsValid` _thwompstart
          (:`Is Valid`
            (`/Engine/EditorBlueprintResources/StandardMacros.IsValid` _thwompend
              (:`Is Valid`
                (`SceneComponent.K2_SetWorldTransform` (`self.thwomp`) (`|EaseFunction` "EaseIn" (`self.AlphaFall`) (`SceneComponent.K2_GetComponentToWorld` _thwompstart) (`SceneComponent.K2_GetComponentToWorld` _thwompend)) true false))
              (:`Is Not Valid`
                (`KismetSystemLibrary.PrintString` "Object Not Set" :!label _label_3))))
          (:`Is Not Valid`
            (goto _label_3))))
      (:`Finished`
        (set `self.IsFalling` false)))))

(event `self.ThwompHurtbox.OnComponentBeginOverlap`
  (params (OverlappedComponent :type "PrimitiveComponent Object Reference") (OtherActor :type "Actor Object Reference") (OtherComp :type "PrimitiveComponent Object Reference") (OtherBodyIndex :type Integer) (bFromSweep :type Boolean) (SweepResult :type "HitResult Structure (by ref)"))
  (bind _as_bp_side_scroller_character (`self.As BP Side Scroller Character`))
  ;[0.15 0.005781 0.005781 0.5] If Hurtbox touches player character, character is squishes, loses health, then is returned to normal
  (bind _asbp_side_scroller_character (cast `/Game/Blueprints/BP_SideScrollerCharacter` OtherActor)
    (:`then`
      (bind _output_get (set `self.As BP Side Scroller Character` _asbp_side_scroller_character))
      (`self.SetActorRelativeScale3D` _output_get (1.5 1.5 0.5))
      (`KismetSystemLibrary.Delay` 2.0)
      (`/Game/Blueprints/BP_GameInstance.TakeDamage` (`self.As BP Game Instance`))
      (set `/Game/Blueprints/BP_SideScrollerCharacter.HasFireFlower` false _as_bp_side_scroller_character)
      (`self.SetActorScale3D` _as_bp_side_scroller_character (1.0 1.0 1.0)))
    (:`CastFailed`
      (`KismetSystemLibrary.PrintString` "cast failed"))))

(fn `UserConstructionScript`)