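; BP_Star is a power-up pickup for the side-scroller character, apparently an invincibility-style star.
; When the character overlaps its box, it calls that character's StarAbility and destroys itself, so the effect itself lives in the character.
; It also caches the game instance on BeginPlay without using it, and holds an unfinished, unconnected timeline meant to tint the player mesh in rainbow colors.
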(event `self.ReceiveBeginPlay`
  ;[0.15 0.005781 0.005781 0.5] Get Game Instance Ref
  (bind _asbp_game_instance (cast `/Game/Blueprints/BP_GameInstance` (`GameplayStatics.GetGameInstance`)))
  (set `self.As BP Game Instance` _asbp_game_instance))

(event `self.Box.OnComponentBeginOverlap`
  (params (OverlappedComponent :type "PrimitiveComponent Object Reference") (OtherActor :type "Actor Object Reference") (OtherComp :type "PrimitiveComponent Object Reference") (OtherBodyIndex :type Integer) (bFromSweep :type Boolean) (SweepResult :type "HitResult Structure (by ref)"))
  ;[0.15 0.005781 0.005781 0.5] When Player Overlaps, run Star Ability code in Player, then destroy self
  (bind _asbp_side_scroller_character (cast `/Game/Blueprints/BP_SideScrollerCharacter` OtherActor))
  (bind _output_get (set `self.As BP Side Scroller Character` _asbp_side_scroller_character))
  (`/Game/Blueprints/BP_SideScrollerCharacter.Star Ability` _output_get)
  (`self.K2_DestroyActor`))

(fn `UserConstructionScript`)