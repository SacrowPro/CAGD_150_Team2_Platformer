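; BP_DeathZone is a hazard volume that penalizes and respawns the side-scroller character when it overlaps the Deathbox component.
; On overlap it sets Health to 1 on BP_GameInstance, then calls TakeDamage after a two-second delay.
; After another second it calls ReduceSize on the game instance and moves the character to its stored RespawnPoint.
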(event `self.Deathbox.OnComponentBeginOverlap`
  (params (OverlappedComponent :type "PrimitiveComponent Object Reference") (OtherActor :type "Actor Object Reference") (OtherComp :type "PrimitiveComponent Object Reference") (OtherBodyIndex :type Integer) (bFromSweep :type Boolean) (SweepResult :type "HitResult Structure (by ref)"))
  (bind _asbp_side_scroller_character (cast `/Game/Blueprints/BP_SideScrollerCharacter` OtherActor))
  (set `self.SideScrollerRef` _asbp_side_scroller_character)
  (bind _asbp_game_instance (cast `/Game/Blueprints/BP_GameInstance` (`GameplayStatics.GetGameInstance`)))
  (set `self.GameInstanceRef` _asbp_game_instance)
  (set `/Game/Blueprints/BP_GameInstance.Health` 1 (`self.GameInstanceRef`))
  (`KismetSystemLibrary.Delay` 2.0)
  (`/Game/Blueprints/BP_GameInstance.TakeDamage` (`self.GameInstanceRef`))
  (`KismetSystemLibrary.Delay` 1.0)
  (`/Game/Blueprints/BP_GameInstance.ReduceSize` (`self.GameInstanceRef`))
  (`self.K2_SetActorLocation` (`self.SideScrollerRef`) (`/Game/Blueprints/BP_SideScrollerCharacter.RespawnPoint` (`self.SideScrollerRef`)) false false))

(fn `UserConstructionScript`)