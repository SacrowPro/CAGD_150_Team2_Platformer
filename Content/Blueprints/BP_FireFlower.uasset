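; Fire flower power-up pickup for the side-scroller character.
; On begin play it caches the game instance.
; When the player character overlaps it, it sets game instance health to 2, scales the character to its big size, sets its fire flower flag and destroys itself.
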(event `self.ReceiveBeginPlay`
  ;[0.15 0.005781 0.005781 0.5] Get Game Instance Ref
  (bind _asbp_game_instance (cast `/Game/Blueprints/BP_GameInstance` (`GameplayStatics.GetGameInstance`)))
  (set `self.As BP Game Instance` _asbp_game_instance))

(event `self.ReceiveActorBeginOverlap`
  (params (OtherActor :type "Actor Object Reference"))
  (bind _as_bp_side_scroller_character (`self.As BP Side Scroller Character`))
  ; Change the players size upon collision destroy after player collides
  (bind _asbp_side_scroller_character (cast `/Game/Blueprints/BP_SideScrollerCharacter` OtherActor))
  (set `self.As BP Side Scroller Character` _asbp_side_scroller_character)
  (set `/Game/Blueprints/BP_GameInstance.Health` 2 (`self.As BP Game Instance`))
  (`self.SetActorScale3D` _as_bp_side_scroller_character (`/Game/Blueprints/BP_SideScrollerCharacter.BigSize` _as_bp_side_scroller_character))
  (set `/Game/Blueprints/BP_SideScrollerCharacter.HasFireFlower` true _as_bp_side_scroller_character)
  (`self.K2_DestroyActor`))

(fn `UserConstructionScript`)