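; Base side-scroller enemy that walks forward, turns around on its Hit event, hurts the player on contact and can be stomped.
; Capsule hits near the HitSpot component bounce the player upward, disable the enemy's hurt box and collision, squash its mesh, then destroy it after a delay.
; HurtBox overlaps knock the player back against their velocity and call TakeDamage on BP_GameInstance, which holds Health, while health remains.
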(event `self.ReceiveTick`
  (params (DeltaSeconds :type "Float (single-precision)"))
  (`self.AddMovementInput` (`self.GetActorForwardVector`) (* DeltaSeconds (`self.Speed`))))

(event `self.CapsuleComponent.OnComponentHit`
  (params (HitComponent :type "PrimitiveComponent Object Reference") (OtherActor :type "Actor Object Reference") (OtherComp :type "PrimitiveComponent Object Reference") (NormalImpulse :type "Vector Structure") (Hit :type "HitResult Structure (by ref)"))
  (bind _mesh (`self.Mesh`))
  (bind (_relativescale3d_x _relativescale3d_y _relativescale3d_z) (`KismetMathLibrary.BreakVector` (`SceneComponent.RelativeScale3D` _mesh)))
  ; The capsule component hit action
  ; If the scene component was hit, then it launched the character by 400 units on the Z axis. They keep momentum and target direction.
  (if (== (`.ImpactPoint` (`GameplayStatics.BreakHitResult` Hit)) (`SceneComponent.K2_GetComponentLocation` (`self.HitSpot`)) :`ErrorTolerance` 50.0)
    (bind _asbp_side_scroller_character (cast `/Game/Blueprints/BP_SideScrollerCharacter` OtherActor))
    (`self.LaunchCharacter` _asbp_side_scroller_character (0.0 0.0 400.0) false false)
    ; Sets collision to none on the capsule, then squishes the character to half scale before destroying the actor.
    (`ActorComponent.K2_DestroyComponent` (`self.HurtBox`))
    (`PrimitiveComponent.SetCollisionEnabled` (`self.CapsuleComponent`) "NoCollision")
    (`SceneComponent.SetRelativeScale3D` _mesh (`KismetMathLibrary.MakeVector` _relativescale3d_x _relativescale3d_y (/ _relativescale3d_z 2.0)))
    (`SceneComponent.K2_AddLocalOffset` (`self.Mesh`) (0.0 0.0 -55.0) false true)
    (`KismetSystemLibrary.K2_SetTimerDelegate` (delegate `Squished`) 1.0)))

(event `Squished`
  ; Sets collision to none on the capsule, then squishes the character to half scale before destroying the actor.
  (`self.K2_DestroyActor`))

(event `self.ReceiveBeginPlay`
  ;[0.15 0.005781 0.005781 0.5] Get reference to BP_GameInstance
  (bind _asbp_game_instance (cast `/Game/Blueprints/BP_GameInstance` (`GameplayStatics.GetGameInstance`)))
  (set `self.GameInstanceRef` _asbp_game_instance))

(event `self.ReceiveHit`
  (params (MyComp :type "PrimitiveComponent Object Reference") (Other :type "Actor Object Reference") (OtherComp :type "PrimitiveComponent Object Reference") (bSelfMoved :type Boolean) (HitLocation :type "Vector Structure") (HitNormal :type "Vector Structure") (NormalImpulse :type "Vector Structure") (Hit :type "HitResult Structure (by ref)"))
  (`self.Turn`))

(event `self.HurtBox.OnComponentBeginOverlap`
  (params (OverlappedComponent :type "PrimitiveComponent Object Reference") (OtherActor :type "Actor Object Reference") (OtherComp :type "PrimitiveComponent Object Reference") (OtherBodyIndex :type Integer) (bFromSweep :type Boolean) (SweepResult :type "HitResult Structure (by ref)"))
  (bind _returnvalue_x (`KismetMathLibrary.BreakVector` (* 2.0 (* (`self.GetVelocity` (`self.SideScrollerRef`)) -1.0))))
  ; Knock Back code
  (bind _asbp_side_scroller_character (cast `/Game/Blueprints/BP_SideScrollerCharacter` OtherActor))
  (bind _output_get (set `self.SideScrollerRef` _asbp_side_scroller_character))
  (if (> (`/Game/Blueprints/BP_GameInstance.Health` (`self.GameInstanceRef`)) 0)
    (`self.LaunchCharacter` _output_get (`KismetMathLibrary.MakeVector` _returnvalue_x 0.0 200.0) false false)
    ;[0.15 0.005781 0.005781 0.5] Call Take Damage Event from Game Instance
    (`/Game/Blueprints/BP_GameInstance.TakeDamage` (`self.GameInstanceRef`))))

(fn `Turn`
  (`self.K2_SetActorRotation` (`KismetMathLibrary.ComposeRotators` (`self.K2_GetActorRotation`) (struct :`Yaw` 180.0))))

(fn `UserConstructionScript`)