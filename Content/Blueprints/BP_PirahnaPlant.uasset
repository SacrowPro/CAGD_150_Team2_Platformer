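; BP_PirahnaPlant is a Piranha Plant hazard that moves back and forth from its placed location and hurts the side-scroller player on touch.
; A Timeline offsets the actor from its start location, alternating forward and reverse playback in an endless loop.
; Capsule overlap with BP_SideScrollerCharacter calls TakeDamage and ReduceSize on BP_GameInstance.
; A DoOnce with no reset limits this to one hit per plant instance.
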(event `self.ReceiveBeginPlay`
  ; Pirahna Plant Movement
  (set `self.StartLocation` (`self.K2_GetActorLocation`))
  (`self.MovePlatformToEnd`))

(event `MovePlatformToEnd`
  ; Pirahna Plant Movement
  (bind (_direction _plantmove) (`Timeline|Timeline` :!via `PlayFromStart` :!label _label)
    (:`Update`
      (`self.K2_SetActorLocation` (+ (`self.StartLocation`) _plantmove)))
    (:`Finished`
      (switch `ETimelineDirection` _direction
        (:`Forward`
          (`self.MovePlatformToStart`))
        (:`Backward`
          (`self.MovePlatformToEnd`))))))

(event `MovePlatformToStart`
  ; Pirahna Plant Movement
  (goto _label :!via `ReverseFromEnd`))

(event `self.CapsuleComponent.OnComponentBeginOverlap`
  (params (OverlappedComponent :type "PrimitiveComponent Object Reference") (OtherActor :type "Actor Object Reference") (OtherComp :type "PrimitiveComponent Object Reference") (OtherBodyIndex :type Integer) (bFromSweep :type Boolean) (SweepResult :type "HitResult Structure (by ref)"))
  ; When player touches Piranha Plant, deal damage
  (bind _asbp_side_scroller_character (cast `/Game/Blueprints/BP_SideScrollerCharacter` OtherActor))
  (set `self.As BP Side Scroller Character` _asbp_side_scroller_character)
  (bind _asbp_game_instance (cast `/Game/Blueprints/BP_GameInstance` (`GameplayStatics.GetGameInstance`)))
  (bind _output_get (set `self.As BP Game Instance` _asbp_game_instance))
  (`/Engine/EditorBlueprintResources/StandardMacros.DoOnce` false
    (:`Completed`
      (`/Game/Blueprints/BP_GameInstance.TakeDamage` _output_get)
      (`/Game/Blueprints/BP_GameInstance.ReduceSize` (`self.As BP Game Instance`)))))

(fn `UserConstructionScript`)