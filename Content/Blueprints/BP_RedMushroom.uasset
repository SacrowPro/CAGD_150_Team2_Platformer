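; BP_RedMushroom is a moving power-up pickup for the side-scroller character that makes the player big.
; Tick sweeps it along its move direction at its item speed, and a Hit event reverses that direction.
; On overlap with BP_SideScrollerCharacter, it sets Health to 2 in BP_GameInstance, scales the character up to the BigMode size, then destroys itself.
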(event `self.ReceiveTick`
  (params (DeltaSeconds :type "Float (single-precision)"))
  ; Working on this.
  (`self.K2_AddActorWorldOffset` (* DeltaSeconds (`self.SPeedItem`) (`self.MoveDirection`)) true))

(event `self.ReceiveBeginPlay`
  ;[0.15 0.005781 0.005781 0.5] Get reference to Game Instance
  (bind _asbp_game_instance (cast `/Game/Blueprints/BP_GameInstance` (`GameplayStatics.GetGameInstance`)))
  (set `self.As BP Game Instance` _asbp_game_instance))

(event `self.ReceiveActorBeginOverlap`
  (params (OtherActor :type "Actor Object Reference"))
  ; Change the players size upon collision destroy after player collides
  (bind _asbp_side_scroller_character (cast `/Game/Blueprints/BP_SideScrollerCharacter` OtherActor))
  (set `self.As BP Side Scroller Character` _asbp_side_scroller_character)
  (set `/Game/Blueprints/BP_GameInstance.Health` 2 (`self.As BP Game Instance`))
  (`self.SetActorScale3D` (`self.As BP Side Scroller Character`) (`self.BigMode`))
  (`self.K2_DestroyActor`))

(event `self.ReceiveHit`
  (params (MyComp :type "PrimitiveComponent Object Reference") (Other :type "Actor Object Reference") (OtherComp :type "PrimitiveComponent Object Reference") (bSelfMoved :type Boolean) (HitLocation :type "Vector Structure") (HitNormal :type "Vector Structure") (NormalImpulse :type "Vector Structure") (Hit :type "HitResult Structure (by ref)"))
  (set `self.MoveDirection` (* -1.0 (`self.MoveDirection`))))

(fn `UserConstructionScript`)