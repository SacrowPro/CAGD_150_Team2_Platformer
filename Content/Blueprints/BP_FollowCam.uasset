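; BP_FollowCam is a follow camera actor for the side-scroller player character.
; It caches the character on BeginPlay, then each Tick moves to the player's location plus an Offset, only while that target's Z stays above a fixed floor, otherwise holding position.
; The construction script previews placement in the editor using the level's character, but checks the character's own height rather than the offset position.
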(event `self.ReceiveBeginPlay`
  ; stores a reference to the player object
  (bind _asbp_side_scroller_character (cast `/Game/Blueprints/BP_SideScrollerCharacter` (`GameplayStatics.GetPlayerCharacter` 0)))
  (set `self.PlayerRef` _asbp_side_scroller_character))

(event `self.ReceiveTick`
  (params (DeltaSeconds :type "Float (single-precision)"))
  (bind _returnvalue (+ (`self.K2_GetActorLocation` (`self.PlayerRef`)) (`self.Offset`)))
  ; sets the players camera plus an offset each frame.
  (if (>= (.z _returnvalue) 160.0)
    (`self.K2_SetActorLocation` _returnvalue)))

(fn `UserConstructionScript`
  ; Sets the camera in the editor whenever the offset changes.
  (bind _returnvalue (`GameplayStatics.GetActorOfClass` "/Game/Blueprints/BP_SideScrollerCharacter.BP_SideScrollerCharacter_C"))
  (bind _returnvalue_2 (`self.K2_GetActorLocation` _returnvalue))
  (if (>= (.z _returnvalue_2) 160.0)
    (`self.K2_SetActorLocation` (+ _returnvalue_2 (`self.Offset`)))))