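; BP_TestMushroom is a test mushroom pickup actor that reacts to overlaps and references the side-scroller character.
; On overlap it casts its own Player variable, not the overlapping actor, to BP_SideScrollerCharacter and stops if that fails.
; On success it stores the result back in Player, calls the empty OnPickUp event and sets its own scale to a large fixed size.
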(event `self.ReceiveActorBeginOverlap`
  (params (OtherActor :type "Actor Object Reference"))
  (`parent.ReceiveActorBeginOverlap` OtherActor)
  (bind _asbp_side_scroller_character (cast `/Game/Blueprints/BP_SideScrollerCharacter` (`self.Player`)))
  (set `self.Player` _asbp_side_scroller_character)
  (`self.On Pick Up`)
  (`self.SetActorScale3D` (10.0 10.0 10.0)))

(event `self.On Pick Up`)

(fn `UserConstructionScript`
  (`parent.UserConstructionScript`))