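; BP_EndGoal is the level-end flag for a side-scroller that finishes the level when the player character hits it.
; On hit, it disables the character's movement and plays a Timeline that eases the flag linearly from FlagStart to FlagEnd, printing a warning if either is invalid.
; When the Timeline finishes, it waits briefly and opens NextLevelToOpen.
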(event `self.ReceiveHit`
  (params (MyComp :type "PrimitiveComponent Object Reference") (Other :type "Actor Object Reference") (OtherComp :type "PrimitiveComponent Object Reference") (bSelfMoved :type Boolean) (HitLocation :type "Vector Structure") (HitNormal :type "Vector Structure") (NormalImpulse :type "Vector Structure") (Hit :type "HitResult Structure (by ref)"))
  (bind _flagstart (`self.FlagStart`))
  (bind _flagend (`self.FlagEnd`))
  ;[0.15 0.005781 0.005781 0.5] When Player reaches the endgoal, flag moves down
  (bind _asbp_side_scroller_character (cast `/Game/Blueprints/BP_SideScrollerCharacter` Other))
  (bind _output_get (set `self.As BP Side Scroller Character` _asbp_side_scroller_character))
  (`CharacterMovementComponent.DisableMovement` (`Character.CharacterMovement` _output_get))
  (bind (_direction _alphaflag) (`Timeline|Timeline`)
    (:`Update`
      (set `self.Alpha Flag` _alphaflag)
      (`/Engine/EditorBlueprintResources/StandardMacros.IsValid` _flagstart
        (:`Is Valid`
          (`/Engine/EditorBlueprintResources/StandardMacros.IsValid` _flagend
            (:`Is Valid`
              (`SceneComponent.K2_SetWorldTransform` (`self.Flag`) (`|EaseFunction` "Linear" (`self.Alpha Flag`) (`SceneComponent.K2_GetComponentToWorld` _flagstart) (`SceneComponent.K2_GetComponentToWorld` _flagend)) true false))
            (:`Is Not Valid`
              (`KismetSystemLibrary.PrintString` "Object Not Set" :!label _label))))
        (:`Is Not Valid`
          (goto _label))))
    (:`Finished`
      ;[0.15 0.005781 0.005781 0.5] When Flag reaches end, load the next level
      (`KismetSystemLibrary.Delay` 0.2)
      (`GameplayStatics.OpenLevelBySoftObjectPtr` (`self.NextLevelToOpen`)))))

(fn `UserConstructionScript`)