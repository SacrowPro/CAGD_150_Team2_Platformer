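; Fireball projectile actor for a side-scroller, meant to fly horizontally in the direction the player faces.
; On its first tick it reads the player character's yaw once, choosing +X for zero yaw and -X otherwise.
; Each tick applies an unswept world offset built from speed and normalized direction, though a zero-vector factor makes that offset zero as written.
; It contains no hit or damage logic.
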(event `self.ReceiveTick`
  (params (DeltaSeconds :type "Float (single-precision)"))
  (`|ExecutionSequence`
    (:`then_0`
      (`self.DetermineDirection`))
    (:`then_1`
      (`self.K2_AddActorWorldOffset` (* (0.0 0.0 0.0) (`self.FireballMoveSpeed`) (`KismetMathLibrary.Normal` (`self.FireballMoveDirection`)))))))

(event `DetermineDirection`
  (bind (_returnvalue_roll _returnvalue_pitch _returnvalue_yaw) (`KismetMathLibrary.BreakRotator` (`self.K2_GetActorRotation` (`self.PlayerCharacterRef`))))
  ;[0.15 0.005781 0.005781 0.5] Detemines which way the fireball's shoot direction is based on player rotation
  (`/Engine/EditorBlueprintResources/StandardMacros.DoOnce` false
    (:`Completed`
      (bind _asbp_side_scroller_character (cast `/Game/Blueprints/BP_SideScrollerCharacter` (`GameplayStatics.GetPlayerPawn` 0)))
      (set `self.PlayerCharacterRef` _asbp_side_scroller_character)
      (if (== _returnvalue_yaw 0.0)
        (set `self.FireballMoveDirection` (1.0 0.0 0.0))
        (else
          (set `self.FireballMoveDirection` (-1.0 0.0 0.0)))))))

(fn `UserConstructionScript`)